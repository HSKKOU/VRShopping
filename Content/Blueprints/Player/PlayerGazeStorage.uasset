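; Player gaze logger that buffers gaze samples and posts them to a web endpoint as JSON.
; AddGazeInfo skips samples matching the last one's item and user position, otherwise stamping the previous entry with its elapsed time before appending.
; A one-second loop from BeginPlay calls SendGazeInfo, which moves all but the newest, still-open entry into the request.
; Responses and failures are only printed, and userId is fixed at zero.
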(event `self.ReceiveBeginPlay`
  (`|ExecutionSequence` :!label _label
    (:`then_0`
      (if (> (`KismetArrayLibrary.Array_Length` (`self.GazeInfos`)) 0)
        (`self.SendGazeInfo`)))
    (:`then_1`
      (`KismetSystemLibrary.Delay` 1.0)
      (goto _label))))

(event `SendGazeInfo`
  (set `self.Request` (`VaRestRequestJSON.ConstructRequestExt` "POST" "json"))
  (add `VaRestRequestJSON.OnRequestComplete` (`self.Request`) (delegate `OnComplete`))
  (add `VaRestRequestJSON.OnRequestFail` (`self.Request`) (delegate `OnFail`))
  (bind _json (`self.createGazeInfoJson` (`self.popGazeInfo`)))
  (if (> (`KismetArrayLibrary.Array_Length` _json) 0)
    (bind _output_get (set `self.SendJsonObject` (`VaRestJsonObject.ConstructJsonObject`)))
    (`VaRestJsonObject.SetObjectArrayField` _output_get "inputs" _json)
    (`VaRestJsonObject.SetNumberField` (`self.SendJsonObject`) "userId" 0.0)
    (`VaRestRequestJSON.SetRequestObject` (`self.Request`) (`self.SendJsonObject`))
    (`VaRestRequestJSON.ProcessURL` (`self.Request`) (`self.postGazeInputURL`))))

(event `OnComplete`
  (params (Request :type "VaRestRequestJSON Object Reference"))
  (`KismetSystemLibrary.PrintString` (`VaRestRequestJSON.ResponseContent` Request)))

(event `OnFail`
  (params (Request :type "VaRestRequestJSON Object Reference"))
  (`KismetSystemLibrary.PrintString` (`VaRestRequestJSON.ResponseContent` Request)))

(fn `AddGazeInfo`
  (params (GazeInfo :type "/Game/Blueprints/Structures/GazeInfo Structure"))
  (bind _gazeinfos (`self.GazeInfos`))
  (bind _gazeinfos_2 (`self.GazeInfos`))
  (bind _returnvalue (`KismetArrayLibrary.Array_LastIndex` _gazeinfos))
  (bind (_userposition _itemid _itemposition _gazepoint _timestamp) (break `/Game/Blueprints/Structures/GazeInfo` (`KismetArrayLibrary.Array_Get` _gazeinfos _returnvalue)))
  (if (> (`KismetArrayLibrary.Array_Length` (`self.GazeInfos`)) 0)
    ;[1 1 1] 前回挿入したものと同じかどうか
    (if (`self.EqualGazeInfo` (`KismetArrayLibrary.Array_Get` _gazeinfos_2 (`KismetArrayLibrary.Array_LastIndex` _gazeinfos_2)) GazeInfo)
      (return)
      (else
        (`KismetArrayLibrary.Array_Set` (`self.GazeInfos`) _returnvalue (make `/Game/Blueprints/Structures/GazeInfo` _userposition _itemid _itemposition _gazepoint _timestamp (`/Game/Blueprints/Macros/ItemMacros.CalcTimeSpan` (`.timestamp_16_39485C394684D71FD4EE369F4F78B083` (break `/Game/Blueprints/Structures/GazeInfo` GazeInfo)) _timestamp)))
        (`KismetArrayLibrary.Array_Add` (`self.GazeInfos`) GazeInfo)
        (return)))
    (else
      ;[1 1 1] 初回
      (`KismetArrayLibrary.Array_Add` (`self.GazeInfos`) GazeInfo)
      (return))))

(fn `createGazeInfoJson`
  (params (PopGazeInfos :type "Array of /Game/Blueprints/Structures/GazeInfo Structure"))
  (returns (Json :type "Array of VaRestJsonObject Object Reference"))
  (locals (GazeInfoJson :type "Array of VaRestJsonObject Object Reference") (gij :type "VaRestJsonObject Object Reference"))
  (for _index (range (+ (`KismetArrayLibrary.Array_LastIndex` PopGazeInfos) 1))
    (bind _output_get (set `local.gij` (`VaRestJsonObject.ConstructJsonObject`)))
    (bind (_userposition _itemid _itemposition _gazepoint _timestamp _pasttime) (break `/Game/Blueprints/Structures/GazeInfo` (`KismetArrayLibrary.Array_Get` PopGazeInfos _index)))
    (`VaRestJsonObject.SetStringField` _output_get "user_positionV3" (`/Game/Blueprints/Macros/ItemMacros.Vector3ToStr` _userposition))
    (`VaRestJsonObject.SetNumberField` _output_get "gaze_item_id" (`KismetMathLibrary.Conv_IntToDouble` _itemid))
    (`VaRestJsonObject.SetStringField` _output_get "gaze_item_positionV3" (`/Game/Blueprints/Macros/ItemMacros.Vector3ToStr` _itemposition))
    (`VaRestJsonObject.SetStringField` _output_get "gaze_pointV2" (`/Game/Blueprints/Macros/ItemMacros.Vector2ToStr` _gazepoint))
    (`VaRestJsonObject.SetStringField` _output_get "gaze_at_time" (`/Game/Blueprints/Macros/ItemMacros.DateToStr` _timestamp))
    (`VaRestJsonObject.SetNumberField` _output_get "time" _pasttime)
    (`KismetArrayLibrary.Array_Add` (`local.GazeInfoJson`) (`local.gij`)))
  (return (`local.GazeInfoJson`)))

(fn `EqualGazeInfo`
  (params (G1 :type "/Game/Blueprints/Structures/GazeInfo Structure") (G2 :type "/Game/Blueprints/Structures/GazeInfo Structure"))
  (returns (`Return Value` :type Boolean))
  (bind (_userposition _itemid) (break `/Game/Blueprints/Structures/GazeInfo` G1))
  (bind (_userposition_2 _itemid_2) (break `/Game/Blueprints/Structures/GazeInfo` G2))
  (return (and (== _itemid _itemid_2) (== _userposition _userposition_2) true)))

(fn `Initialize`)

(fn `popGazeInfo`
  (returns (GazeInfos :type "Array of /Game/Blueprints/Structures/GazeInfo Structure"))
  (locals (SendInfos :type "Array of /Game/Blueprints/Structures/GazeInfo Structure"))
  (bind _item (`KismetArrayLibrary.Array_Get` (`self.GazeInfos`)))
  (if (> (`KismetArrayLibrary.Array_Length` (`self.GazeInfos`)) 1)
    (while (> (`KismetArrayLibrary.Array_Length` (`self.GazeInfos`)) 1)
      (`KismetArrayLibrary.Array_Add` (`local.SendInfos`) _item)
      (`KismetArrayLibrary.Array_RemoveItem` (`self.GazeInfos`) _item))
    (return (`local.SendInfos`))
    (else
      (return (`local.SendInfos`)))))

(fn `UserConstructionScript`)