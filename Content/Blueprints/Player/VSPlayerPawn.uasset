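; Player pawn that moves relative to the camera and records which items the player looks at.
; Axis inputs drive movement and yaw, with separate walk speeds for forward and backward motion.
; Each tick, a short line trace from the camera finds tagged ItemActors and builds timestamped gaze info from player position, item ID and hit point.
; Valid hits are added to a PlayerGazeStorage actor spawned at BeginPlay.
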(event `self.ReceiveBeginPlay`
  (bind _returnvalue (`|SpawnActorFromClass` "/Game/Blueprints/Player/PlayerGazeStorage.PlayerGazeStorage_C" (`KismetMathLibrary.MakeTransform` (0.0 0.0 10000.0)) "Undefined" "OverrideRootScale"))
  (set `self.GazeStorage` _returnvalue))

(event `self.ReceiveTick`
  (params (DeltaSeconds :type "Float (single-precision)"))
  (bind _returnvalue (`GameplayStatics.GetPlayerCameraManager` 0))
  (bind (_x _y) (`KismetMathLibrary.BreakVector2D` (0.0 0.0)))
  (`|ExecutionSequence`
    (:`then_0`
      (`self.AddMovementInput` (+ (* (`self.GetActorRightVector` _returnvalue) _x) (* (`self.GetActorForwardVector` _returnvalue) _y)) 1.0))
    (:`then_1`
      ;[1 1 1] Trace Gaze
      (bind _gazeinfo (`self.TraceGazePoint`))
      (if (> (`.itemId_7_28817EF14F9C7FDAA461BD92D2C05B11` (break `/Game/Blueprints/Structures/GazeInfo` _gazeinfo)) 0)
        (`/Game/Blueprints/Player/PlayerGazeStorage.AddGazeInfo` (`self.GazeStorage`) _gazeinfo)))))

(event `InputAxis|MoveForward`
  (params (AxisValue :type "Float (single-precision)"))
  (bind _charactermovement (`self.CharacterMovement`))
  ;[1 1 1] Movement
  (`|ExecutionSequence`
    (:`then_0`
      (if (> AxisValue 0.0)
        (set `CharacterMovementComponent.MaxWalkSpeed` (`self.ForwardSpeed`) _charactermovement)
        (else
          (set `CharacterMovementComponent.MaxWalkSpeed` (`self.BackSpeed`) _charactermovement))))
    (:`then_1`
      (`self.AddMovementInput` (`self.GetActorForwardVector` (`GameplayStatics.GetPlayerCameraManager` 0)) AxisValue))))

(event `InputAxis|MoveRight`
  (params (AxisValue :type "Float (single-precision)"))
  ;[1 1 1] Movement
  (`self.AddMovementInput` (`self.GetActorRightVector` (`GameplayStatics.GetPlayerCameraManager` 0)) AxisValue))

(event `InputAxis|LookRight`
  (params (AxisValue :type "Float (single-precision)"))
  ;[1 1 1] Movement
  (`self.AddControllerYawInput` AxisValue))

(fn `TraceGazePoint`
  (returns (GazeInfo :type "/Game/Blueprints/Structures/GazeInfo Structure"))
  (bind _returnvalue (`GameplayStatics.GetPlayerCameraManager` 0))
  (bind _returnvalue_2 (`self.K2_GetActorLocation` _returnvalue))
  (bind (_outhit _returnvalue_3) (`KismetSystemLibrary.LineTraceSingle` :`Start` _returnvalue_2 :`End` (+ _returnvalue_2 (* (`self.GetActorForwardVector` _returnvalue) 200.0)) :`TraceChannel` "TraceTypeQuery3" :`DrawDebugType` "ForOneFrame"))
  (if _returnvalue_3
    (bind (_bblockinghit _binitialoverlap _time _location _impactpoint _normal _impactnormal _physmat _hitactor) (`GameplayStatics.BreakHitResult` _outhit))
    (if (`self.ActorHasTag` _hitactor "Item")
      (bind _asitem_actor (cast `/Game/Blueprints/Item/ItemActor` _hitactor)
        (:`then`
          (bind _iteminfo (`/Game/Blueprints/Item/ItemActor.getItemInfo` _asitem_actor))
          (return (make `/Game/Blueprints/Structures/GazeInfo` (`self.K2_GetActorLocation`) (`.id_2_760F7F3D4BCF41CDBAC1F2A64B15FA81` (break `/Game/Blueprints/Structures/ItemInfo` _iteminfo)) _location (0.0 0.0) (`KismetMathLibrary.Now`))))
        (:`CastFailed`
          (return)))
      (else
        _)))
  (return))

(fn `UserConstructionScript`)