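; ItemActor is an item actor that displays an item's picture, fetched from a URL, on its Board component.
; SetItemInfo stores the item info, which GetItemInfo returns, and passes its image URL to LoadImage.
; LoadImage downloads the image, falling back to a default on failure.
; SetItemImage creates a dynamic instance of the item material on Board and sets the texture as its ItemImage parameter.
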(event `self.ReceiveBeginPlay`)

(event `LoadImage`
  (params (ImageURL :type String))
  (bind _texture (`AsyncTaskDownloadImage.DownloadImage` ImageURL)
    (:`OnSuccess`
      (`self.SetItemImage` _texture))
    (:`OnFail`
      (`self.SetItemImage` (`self.DefaultItemImage`)))))

(fn `getItemInfo`
  (returns (ItemInfo :type "/Game/Blueprints/Structures/ItemInfo Structure"))
  (return (`self.ItemInfo`)))

(fn `SetItemImage`
  (params (Value :type "Texture Object Reference"))
  (bind _returnvalue (`PrimitiveComponent.CreateDynamicMaterialInstance` (`self.Board`) 0 "/Game/Resources/Materials/ItemActorMaterial.ItemActorMaterial"))
  (`MaterialInstanceDynamic.SetTextureParameterValue` _returnvalue "ItemImage" Value)
  (return))

(fn `SetItemInfo`
  (params (ItemInfo :type "/Game/Blueprints/Structures/ItemInfo Structure"))
  (bind _output_get (set `self.ItemInfo` ItemInfo))
  (`self.LoadImage` (`.url_image_17_6CA2BF38429FABC1937C229D20114C43` (break `/Game/Blueprints/Structures/ItemInfo` _output_get)))
  (return))

(fn `UserConstructionScript`)