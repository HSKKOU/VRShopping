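; ItemManager is a manager Blueprint that loads shop-style item data over HTTP and displays it as actors in the world.
; BeginPlay spawns an ItemStorage actor and binds a GET request, but the ProcessURL call is disconnected, so the request is never sent.
; On completion, JSON entries become ItemInfo structs in storage, then DisplayItems spawns an ItemActor for each in a row along Y.
; Failures only print messages.
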(event `self.ReceiveBeginPlay`
  (bind _returnvalue (`|SpawnActorFromClass` "/Game/Blueprints/Item/ItemStorage.ItemStorage_C" (`KismetMathLibrary.MakeTransform` (0.0 0.0 1000.0)) "Undefined" "OverrideRootScale"))
  (bind _output_get (set `self.ItemStorage` _returnvalue))
  (`/Game/Blueprints/Item/ItemStorage.Initialize` _output_get)
  (bind _output_get_2 (set `self.ItemsRequest` (`VaRestRequestJSON.ConstructRequestExt` "GET" "x_www_form_urlencoded_url")))
  (add `VaRestRequestJSON.OnRequestComplete` _output_get_2 (delegate `OnComplete`))
  (add `VaRestRequestJSON.OnRequestFail` _output_get_2 (delegate `OnFail`))
  (`KismetSystemLibrary.PrintString` "Get Items"))

(event `OnComplete`
  (params (Request :type "VaRestRequestJSON Object Reference"))
  (`self.OnCompleteLoadItems` Request)
  (`self.DisplayItems`))

(event `OnFail`
  (params (Request :type "VaRestRequestJSON Object Reference"))
  (`KismetSystemLibrary.PrintString` (`VaRestRequestJSON.ResponseContent` Request)))

(fn `CreateItemActor`
  (params (ItemInfo :type "/Game/Blueprints/Structures/ItemInfo Structure") (Transform :type "Transform Structure"))
  (returns (ItemActor :type "/Game/Blueprints/Item/ItemActor Object Reference"))
  (bind _returnvalue (`|SpawnActorFromClass` "/Game/Blueprints/Item/ItemActor.ItemActor_C" Transform "Undefined" "OverrideRootScale"))
  (`/Game/Blueprints/Item/ItemActor.SetItemInfo` _returnvalue ItemInfo)
  (return _returnvalue))

(fn `CreateItemInfo`
  (params (Items :type "VaRestJsonObject Object Reference"))
  (returns (ItemInfo :type "/Game/Blueprints/Structures/ItemInfo Structure"))
  (return (make `/Game/Blueprints/Structures/ItemInfo` (`KismetStringLibrary.Conv_StringToInt` (`VaRestJsonObject.GetStringField` Items "id")) (`VaRestJsonObject.GetStringField` Items "item_code") (`VaRestJsonObject.GetStringField` Items "name") (`KismetStringLibrary.Conv_StringToInt` (`VaRestJsonObject.GetStringField` Items "price")) (`VaRestJsonObject.GetStringField` Items "description") (`VaRestJsonObject.GetStringField` Items "url_item") (`VaRestJsonObject.GetStringField` Items "url_image") (`KismetStringLibrary.Conv_StringToInt` (`VaRestJsonObject.GetStringField` Items "review_num")) (`KismetStringLibrary.Conv_StringToDouble` (`VaRestJsonObject.GetStringField` Items "review_avg")) (`KismetStringLibrary.Conv_StringToInt` (`VaRestJsonObject.GetStringField` Items "genre_id")))))

(fn `DisplayItems`
  (for _index (range (+ (`/Game/Blueprints/Item/ItemStorage.LastItemIndex` (`self.ItemStorage`)) 1))
    (`self.CreateItemActor` (`/Game/Blueprints/Item/ItemStorage.GetItem` (`self.ItemStorage`) _index) (`KismetMathLibrary.MakeTransform` (`KismetMathLibrary.MakeVector` 100.0 (* _index 50.0) 112.0))))
  (return))

(fn `OnCompleteLoadItems`
  (params (Request :type "VaRestRequestJSON Object Reference"))
  (bind _returnvalue (`VaRestRequestJSON.GetResponseObject` Request))
  (if (`VaRestJsonObject.GetBoolField` _returnvalue "result")
    (bind _returnvalue_2 (`VaRestJsonObject.GetArrayField` _returnvalue "data"))
    (for _array_element _returnvalue_2
      (bind _returnvalue_3 (`VaRestJsonValue.AsObject` _array_element))
      (bind _iteminfo (`self.CreateItemInfo` _returnvalue_3))
      (`/Game/Blueprints/Item/ItemStorage.AddItem` (`self.ItemStorage`) _iteminfo))
    (return)
    (else
      (`KismetSystemLibrary.PrintString` "Failed to load Items")
      (return))))

(fn `UserConstructionScript`)