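; ItemMacros is a utility library of conversion helpers for vectors and dates.
; Vector2 and Vector3 become comma-separated strings, and DateToStr joins dash-separated date and colon-separated time down to milliseconds, with no separator between the two.
; CalcTimeSpan converts the difference of two dates to milliseconds from its hour, minute, second and millisecond components, leaving out whole days.
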(fn `CalcTimeSpan`
  (params (Date :type "DateTime Structure") (Date2 :type "DateTime Structure"))
  (returns (Span :type "Float (double-precision)"))
  (bind (_days _hours _minutes _seconds _milliseconds) (`KismetMathLibrary.BreakTimespan` (- Date Date2)))
  (return (+ (* (+ (* (+ (* _hours 60.0) (`KismetMathLibrary.Conv_IntToDouble` _minutes)) 60.0) (`KismetMathLibrary.Conv_IntToDouble` _seconds)) 1000.0) (`KismetMathLibrary.Conv_IntToDouble` _milliseconds))))

(fn `DateToStr`
  (params (Date :type "DateTime Structure"))
  (returns (Str :type String))
  (bind (_year _month _day _hour _minute _second _millisecond) (`KismetMathLibrary.BreakDateTime` Date))
  (return (`KismetStringLibrary.Concat_StrStr` (`KismetStringLibrary.JoinStringArray` (`|MakeArray` (`KismetStringLibrary.Conv_IntToString` _year) (`KismetStringLibrary.Conv_IntToString` _month) (`KismetStringLibrary.Conv_IntToString` _day)) "-") " " (`KismetStringLibrary.JoinStringArray` (`|MakeArray` (`KismetStringLibrary.Conv_IntToString` _hour) (`KismetStringLibrary.Conv_IntToString` _minute) (`KismetStringLibrary.Conv_IntToString` _second) (`KismetStringLibrary.Conv_IntToString` _millisecond)) ":"))))

(fn `Vector2ToStr`
  (params (Vector2 :type "Vector2D Structure"))
  (returns (Str :type String))
  (bind (_x _y) (`KismetMathLibrary.BreakVector2D` Vector2))
  (return (`KismetStringLibrary.JoinStringArray` (`|MakeArray` (`KismetStringLibrary.Conv_DoubleToString` _x) (`KismetStringLibrary.Conv_DoubleToString` _y)) ",")))

(fn `Vector3ToStr`
  (params (Vector3 :type "Vector Structure"))
  (returns (Str :type String))
  (return (`KismetStringLibrary.JoinStringArray` (`|MakeArray` (`KismetStringLibrary.Conv_DoubleToString` (.x Vector3)) (`KismetStringLibrary.Conv_DoubleToString` (.y Vector3)) (`KismetStringLibrary.Conv_DoubleToString` (.z Vector3))) ",")))